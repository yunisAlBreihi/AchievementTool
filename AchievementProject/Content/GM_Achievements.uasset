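; Game mode that tracks achievement progress for enemies hit and shots fired, and pops up the matching achievement on screen.
; BeginPlay gathers DAB_Achievement data assets from a folder via the Asset Registry, then after a short delay creates a W_Achievement widget for player controller index 1.
; Event entry points update a unique enemy list and a shot counter, showing achievements looked up by asset name when their thresholds match.
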(event Custom|AddEnemyToHitList
  (params (Enemy :type BP%20Test%20Enemy%20Object%20Reference))
  (bind _array_element (Achievement|GetAchievement "DA_KillerOfMany"))
  ;[1 1 1] If an enemy is hit, add to list
  (bind _returnvalue (Utilities|Array|AddUnique (Variables|Achievement|GetEnemiesHit) Enemy))
  (if (== _returnvalue (- (.NeededToComplete (Utilities|Struct|BreakS_Achievement (Variables|/Game/AchievementTool/Assets/DAB_Achievement.DAB_Achievement_C|GetAchievement _array_element))) 1))
    (Default|ShowAchievement (Variables|Achievement|Getachievement_UI) _array_element)))

(event Custom|AddToShotsFired
  (bind _array_element (Achievement|GetAchievement "DA_ShotsFired"))
  ;[1 1 1] Iterates the shots fired variable
  (bind _result (Math|Integer|IncrementInt (Variables|Achievement|GetShotsFired))
    (:%20%20
      (if (== _result (- (.NeededToComplete (Utilities|Struct|BreakS_Achievement (Variables|/Game/AchievementTool/Assets/DAB_Achievement.DAB_Achievement_C|GetAchievement _array_element))) 1))
        (Default|ShowAchievement (Variables|Achievement|Getachievement_UI) _array_element)))))

(event EventBeginPlay
  ;[1 0.4663 0.3664] BeginPlay
  ;;[1 1 1] Get all achievements
  (bind _outassetdata (Class|AssetRegistry|GetAssetsbyPath (Class|AssetRegistryHelpers|GetAssetRegistry) (Variables|Achievement|GetAchievementPath) false false))
  (for _array_element _outassetdata
    (bind _asdab_achievement (Utilities|Casting|CastToDAB_Achievement (Class|AssetRegistryHelpers|GetAsset _array_element)))
    (Utilities|Array|AddUnique (Variables|Achievement|Getachievements) _asdab_achievement))
  ;;[1 1 1] Add AchievementUI to player
  (Utilities|FlowControl|Delay 0.5)
  (bind _returnvalue (UserInterface|CreateWidget "/Game/AchievementTool/UI_Achievement/W_Achievement.W_Achievement_C" (Game|GetPlayerController 1)))
  (bind _output_get (Variables|Achievement|Setachievement_UI _returnvalue))
  (UserInterface|Viewport|AddtoViewport _output_get 0))

(fn ConstructionScript)

(fn GetAchievement
  (params (AchievementDisplayName :type String))
  (for _array_element (Variables|Achievement|Getachievements)
    (if (Utilities|Enum|Equal(Enum) (Utilities|GetDisplayName _array_element) AchievementDisplayName)
      (return _array_element)))
  (return 0))