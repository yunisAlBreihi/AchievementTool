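; BP_Achievement_Save stores achievement data for saving and restores it onto the achievement entries.
; SetAchievements keeps the passed array and appends each entry's Achievement value to a parallel SAchievements array, without clearing it first.
; GetAchievements copies those stored values back into each entry's Achievement by matching index, then returns the Achievements array.
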(fn GetAchievements
  (for (_array_element _array_index) (Variables|Achievements|GetAchievements)
    (Variables|/Game/AchievementTool/Assets/DAB_Achievement.DAB_Achievement_C|SetAchievement _array_element (Utilities|Array|Get(acopy) (Variables|Achievements|GetSAchievements) _array_index)))
  (return (Variables|Achievements|GetAchievements)))

(fn SetAchievements
  (params (Array :type Array%20of%20DAB%20Achievement%20Object%20References))
  (bind _output_get (Variables|Achievements|SetAchievements Array))
  (for _array_element _output_get
    (Utilities|Array|Add (Variables|Achievements|GetSAchievements) (Variables|/Game/AchievementTool/Assets/DAB_Achievement.DAB_Achievement_C|GetAchievement _array_element))))