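; Game mode for the achievement example that tracks progress, shows unlocks on screen and optionally persists them between sessions.
; BeginPlay loads saved achievements via the game instance, falls back to gathering DAB_Achievement assets from a folder through the Asset Registry, then creates the UI widget after a short delay.
; Per-achievement events call TrackAchievement, which finds the asset by name, progresses it and shows it on completion.
; EndPlay writes the array to a save object.
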(event Custom|Ach_JumpKing
  ;[1 0.2033 0.843] Achievement functions
  (CallFunction|TrackAchievement "DA_JumpKing"))

(event Custom|LoadMyData
  ;[0.2257 0.568 1] Save/ Load
  ;;[1 1 1] Load Achievement Data
  (bind _asbp_achievement_game_instance (Utilities|Casting|CastToBP_Achievement_GameInstance (Game|GetGameInstance)))
  (bind _retrievedata (Default|LoadData _asbp_achievement_game_instance (Variables|SaveAchievements|GetSaveDataName)))
  (Utilities|IsValid _retrievedata
    (:Is%20Valid
      (Variables|Achievements|SetAchievements (Default|GetAchievements _retrievedata)))))

(event Custom|SaveMyData
  ;[0.2257 0.568 1] Save/ Load
  ;;[1 1 1] Save Achievement Data
  (bind _asbp_achievement_game_instance (Utilities|Casting|CastToBP_Achievement_GameInstance (Game|GetGameInstance)))
  (bind _returnvalue (SaveGame|CreateSaveGameObject "/Game/AchievementExample/BP_Achievement_Save.BP_Achievement_Save_C"))
  (Default|SetAchievements _returnvalue (Variables|Achievements|GetAchievements))
  (Default|SaveData _asbp_achievement_game_instance _returnvalue (Variables|SaveAchievements|GetSaveDataName) true))

(event Custom|Ach_ShotsFired
  ;[1 0.2033 0.843] Achievement functions
  (CallFunction|TrackAchievement "DA_ShotsFired"))

(event Custom|Ach_KillerOfMany
  ;[1 0.2033 0.843] Achievement functions
  (CallFunction|TrackAchievement "DA_KillerOfMany"))

(event Custom|Ach_Newman
  ;[1 0.2033 0.843] Achievement functions
  (CallFunction|TrackAchievement "DA_Newman"))

(event Custom|Ach_FaceOfDeath
  ;[1 0.2033 0.843] Achievement functions
  (CallFunction|TrackAchievement "DA_FaceOfDeath"))

(event EventBeginPlay
  ;[1 0.4663 0.3664] BeginPlay
  ;;[1 1 1] Load Game when starting the game
  (if (Variables|SaveAchievements|GetbSaveAchievements)
    (CallFunction|LoadMyData))
  ;;[1 1 1] Get all achievements
  (if (== (Utilities|Array|Length (Variables|Achievements|GetAchievements)) 0)
    (bind _outassetdata (Class|AssetRegistry|GetAssetsbyPath (Class|AssetRegistryHelpers|GetAssetRegistry) (Variables|Achievements|GetAchievementPath) false false))
    (for _array_element _outassetdata
      (bind _asdab_achievement (Utilities|Casting|CastToDAB_Achievement (Class|AssetRegistryHelpers|GetAsset _array_element)))
      (Utilities|Array|AddUnique (Variables|Achievements|GetAchievements) _asdab_achievement)))
  ;;[1 1 1] Add AchievementUI to player
  (Utilities|FlowControl|Delay 0.5)
  (bind _returnvalue (UserInterface|CreateWidget "/Game/AchievementTool/UI_Achievement/Widget_UI_Achievement.Widget_UI_Achievement_C" (Game|GetPlayerController 1)))
  (bind _output_get (Variables|Achievements|Setachievement_UI _returnvalue))
  (UserInterface|Viewport|AddtoViewport _output_get 0))

(event EventEndPlay
  (params (EndPlayReason :type EEndPlayReason%20Enum :default "Destroyed"))
  ;[0.2499 1 0.3458] EndPlay
  ;;[1 1 1] Save game when quitting the game
  (if (Variables|SaveAchievements|GetbSaveAchievements)
    (CallFunction|SaveMyData)))

(fn ConstructionScript)

(fn GetAchievement
  (params (AchievementDisplayName :type String))
  (for _array_element (Variables|Achievements|GetAchievements)
    (if (Utilities|Enum|Equal(Enum) (Utilities|GetDisplayName _array_element) AchievementDisplayName)
      (return _array_element)))
  (return 0))

(fn TrackAchievement
  (params (AchievementName :type String))
  (bind _array_element (Achievement|GetAchievement AchievementName))
  (if (not (Default|HasCompleted _array_element))
    (Default|ProgressAchievement _array_element)
    (if (Default|HasCompleted _array_element)
      (Default|ShowAchievement (Variables|Achievements|Getachievement_UI) _array_element))))