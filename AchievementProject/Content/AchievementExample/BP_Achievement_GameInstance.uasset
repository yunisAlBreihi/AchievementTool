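; Game instance for the achievement example that provides save-slot helper functions for storing achievement data.
; LoadData returns the slot's save cast to BP_Achievement_Save, or nothing if the slot is missing or the cast fails.
; SaveData writes to a new slot, replacing an existing one only when Overwrite is set, and DeleteData removes a slot if it exists.
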(fn LoadData
  (params (SlotName :type String))
  (bind _returnvalue (SaveGame|DoesSaveGameExist SlotName))
  (if _returnvalue
    (bind _returnvalue_2 (SaveGame|LoadGamefromSlot SlotName))
    (bind _asbp_achievement_save (Utilities|Casting|CastToBP_Achievement_Save _returnvalue_2)
      (:then
        (return _asbp_achievement_save))
      (:CastFailed
        _)))
  (return 0))

(fn SaveData
  (params (Data :type Save%20Game%20Object%20Reference) (SlotName :type String) (Overwrite :type Boolean))
  (bind _returnvalue (SaveGame|DoesSaveGameExist SlotName))
  (if _returnvalue
    (if Overwrite
      (SaveGame|SaveGametoSlot Data SlotName :!label _label))
    (else
      (goto _label))))

(fn DeleteData
  (params (SlotName :type String))
  (bind _returnvalue (SaveGame|DoesSaveGameExist SlotName))
  (if _returnvalue
    (SaveGame|DeleteGameinSlot SlotName)
    (else
      (return))))