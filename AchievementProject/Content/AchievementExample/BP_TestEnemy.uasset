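; BP_TestEnemy is a test enemy for an achievement example that reports its death to the game mode.
; On BeginPlay it caches a reference to the GM_Achievements game mode.
; When a FirstPersonProjectile hits its static mesh, it sets an IsDead flag so it counts only once, then calls KilledEnemy on the game mode for achievement tracking.
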(event OnComponentHit(StaticMesh)
  (params (HitComponent :type Primitive%20Component%20Object%20Reference) (OtherActor :type Actor%20Object%20Reference) (OtherComp :type Primitive%20Component%20Object%20Reference) (NormalImpulse :type Vector :default "0, 0, 0") (Hit :type Hit%20Result%20Structure%20%28by%20ref%29))
  ;[1 1 1] If hit, add to a hit list on the game mode for achievement tracking
  (if (not (Variables|Default|GetisDead))
    (Utilities|Casting|CastToFirstPersonProjectile OtherActor)
    (Variables|Default|SetisDead true)
    (Default|KilledEnemy (Variables|GameMode|GetGameMode))))

(event EventBeginPlay
  ;[1 0.2493 0.2792] BeginPlay
  (bind _asgm_achievements (Utilities|Casting|CastToGM_Achievements (Game|GetGameMode)))
  (Variables|GameMode|SetGameMode _asgm_achievements))

(fn ConstructionScript)