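; BP_Platform is a one-shot trigger actor in an achievement example that fires the Newman achievement when the first-person character touches it.
; On BeginPlay it caches the GM_Achievements game mode.
; The first FirstPersonCharacter overlap with its Trigger component sets a guard flag, waits briefly, calls AchNewman on that game mode, then destroys the actor.
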(event OnComponentBeginOverlap(Trigger)
  (params (OverlappedComponent :type Primitive%20Component%20Object%20Reference) (OtherActor :type Actor%20Object%20Reference) (OtherComp :type Primitive%20Component%20Object%20Reference) (OtherBodyIndex :type Integer) (bFromSweep :type Boolean) (SweepResult :type Hit%20Result%20Structure%20%28by%20ref%29))
  ;[1 1 1] Trigger Achievement
  (if (not (Variables|Properties|GetbHasTriggered))
    (Utilities|Casting|CastToFirstPersonCharacter OtherActor)
    (Variables|Properties|SetbHasTriggered true)
    (Utilities|FlowControl|Delay 1.0)
    (Default|AchNewman (Variables|GameMode|GetGameMode))
    (Actor|DestroyActor)))

(event EventBeginPlay
  ;[1 0.6612 0.3281] BeginPlay
  (bind _asgm_achievements (Utilities|Casting|CastToGM_Achievements (Game|GetGameMode)))
  (Variables|GameMode|SetGameMode _asgm_achievements))

(fn ConstructionScript)