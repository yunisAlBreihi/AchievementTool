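; BP_BossBox is a boss box in the achievement example that projectiles destroy to unlock the Face of Death achievement.
; It caches GM_Achievements on BeginPlay and decrements Health when its mesh is hit by a FirstPersonProjectile.
; A hit at zero Health drops it to a -1 sentinel that blocks further hits, then after a short delay triggers the achievement through the game mode and destroys the actor.
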(event OnComponentHit(StaticMesh)
  (params (HitComponent :type Primitive%20Component%20Object%20Reference) (OtherActor :type Actor%20Object%20Reference) (OtherComp :type Primitive%20Component%20Object%20Reference) (NormalImpulse :type Vector :default "0, 0, 0") (Hit :type Hit%20Result%20Structure%20%28by%20ref%29))
  ;[1 1 1] When hit five times, will be destroyed and show the Face Of Death achivement.
  (if (!= (Variables|Properties|GetHealth) -1)
    (Utilities|Casting|CastToFirstPersonProjectile OtherActor)
    (if (> (Variables|Properties|GetHealth) 0)
      (Math|Integer|DecrementInt (Variables|Properties|GetHealth))
      (else
        (Math|Integer|DecrementInt (Variables|Properties|GetHealth)
          (:%20%20
            (Utilities|FlowControl|Delay 1.0)
            (Default|AchFaceOfDeath (Variables|GameMode|GetGameMode))
            (Actor|DestroyActor)))))))

(event EventBeginPlay
  ;[1 0.2493 0.2792] BeginPlay
  (bind _asgm_achievements (Utilities|Casting|CastToGM_Achievements (Game|GetGameMode)))
  (Variables|GameMode|SetGameMode _asgm_achievements))

(fn ConstructionScript)